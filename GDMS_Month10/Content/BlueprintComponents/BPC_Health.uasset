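; Health component that tracks its owner's current health as a byte and handles healing, damage and death.
; Healing clamps to max health, while TakeDamage passes through a CanTakeDamage check (always true here) and an Invincible flag.
; Damage subtracts one point per loop step; on finding zero, it fires the Death call, sends DieMessage to the owner and stops.
; A separate Die event fires the Death call directly.
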(event `/Game/Blueprints/BPI_Damage.Die`
  (`self.Death`))

(event `/Game/Blueprints/BPI_Damage.Take Damage`
  (params (IncomingDamage :type Byte) (Source :type "Actor Object Reference"))
  (`self.DecreaseHealth` Source IncomingDamage))

(fn `CanTakeDamage`
  (params (Instigator :type "Actor Object Reference"))
  (returns (Out :type Boolean))
  (return true))

(fn `CheckHealth`
  ;[1 0.1667 0.1846] If Health is at or below 0, call death event
  (if (<= (`self.CurHealth`) 0)
    (`self.Death`)
    (message `/Game/Blueprints/BPI_Damage.Die` (`self.GetOwner`))))

(fn `DecreaseHealth`
  (params (Instigator :type "Actor Object Reference") (Damage :type Byte))
  (bind _out (`self.CanTakeDamage` Instigator))
  (if _out
    ;[1 0.1667 0.1846] Don't reduce health if invincible
    (if (not (`self.Invincible`))
      ;[0.03955 0.4072 0.6584] Incrementally decrease health and check for death
      (for _ (range (+ (`KismetMathLibrary.Conv_ByteToInt` Damage) 1))
        (if (== (`self.CurHealth`) 0)
          (`|ExecutionSequence`
            (:`then_0`
              (`self.CheckHealth`))
            (:`then_1`
              (break)))
          (else
            (set `self.CurHealth` (- (`self.CurHealth`) 1))))))))

(fn `IncreaseHealth`
  (params (UpdateAmount :type Byte))
  ;[0.4397 1 0.402] Add new health to current health. Clamp to max health.
  (set `self.CurHealth` (`KismetMathLibrary.Conv_IntToByte` (`KismetMathLibrary.Clamp` (`KismetMathLibrary.Conv_ByteToInt` (+ (`self.CurHealth`) UpdateAmount)) 0 (`KismetMathLibrary.Conv_ByteToInt` (`self.MaxHealth`))))))
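; Checkpoint banner actor that registers itself with the player on first contact and switches from a closed to an open banner.
; It starts closed, and its capsule overlap filters for actors implementing BPI_Player.
; A DoOnce then prints a debug message, sends the banner through the RegisterCheckpoint interface message and calls ToggleCheckpoint.
; ToggleCheckpoint swaps visibility between the open and closed banner components.
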(event `Toggle Checkpoint`
  (bind _basic_banner_open (`self.Basic_Banner_Open`))
  (bind _basic_banner_closed (`self.Basic_Banner_Closed`))
  (if (`SceneComponent.IsVisible` (`self.Basic_Banner_Open`))
    (`SceneComponent.SetVisibility` _basic_banner_closed true false)
    (`SceneComponent.SetVisibility` _basic_banner_open false false)
    (else
      (`SceneComponent.SetVisibility` _basic_banner_closed false false)
      (`SceneComponent.SetVisibility` _basic_banner_open true false))))

(event `self.ReceiveBeginPlay`
  (`SceneComponent.SetVisibility` (`self.Basic_Banner_Open`) false false)
  (`SceneComponent.SetVisibility` (`self.Basic_Banner_Closed`) true false))

(event `self.Capsule.OnComponentBeginOverlap`
  (params (OverlappedComponent :type "PrimitiveComponent Object Reference") (OtherActor :type "Actor Object Reference") (OtherComp :type "PrimitiveComponent Object Reference") (OtherBodyIndex :type Integer) (bFromSweep :type Boolean) (SweepResult :type "HitResult Structure (by ref)"))
  (if (`KismetSystemLibrary.DoesImplementInterface` OtherActor "/Game/Blueprints/BPI_Player.BPI_Player_C")
    (`/Engine/EditorBlueprintResources/StandardMacros.DoOnce` false
      (:`Completed`
        (`KismetSystemLibrary.PrintString` "Player reach checkpoint")
        (message `/Game/Blueprints/BPI_Player.Register Checkpoint` OtherActor self)
        (`self.Toggle Checkpoint`)))))

(fn `UserConstructionScript`)
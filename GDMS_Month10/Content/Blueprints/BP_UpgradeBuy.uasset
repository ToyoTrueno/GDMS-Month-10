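; BP_UpgradeBuy is a purchasable upgrade pickup for health, attack or blocking movement speed, with floating text showing its coin cost.
; The text is set from Type on BeginPlay and turns toward the player camera every tick.
; A DoOnce-gated capsule overlap deducts the third-person character's coins and passes Type to UpgradePlayerMessage.
; The pickup then hides and reappears after a short delay, while failed purchases reset immediately.
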(event `self.ReceiveBeginPlay`
  (switch `/Game/Blueprints/Upgrades/UpgradeType` (`self.Type`)
    (:`NewEnumerator0`
      (`TextRenderComponent.K2_SetText` (`self.TextRender`) (`KismetTextLibrary.Conv_StringToText` (`KismetStringLibrary.Concat_StrStr` "Health up for: " (`KismetStringLibrary.Conv_IntToString` (`self.Upgrade Cost`)) " Coins"))))
    (:`NewEnumerator1`
      (`TextRenderComponent.K2_SetText` (`self.TextRender`) (`KismetTextLibrary.Conv_StringToText` (`KismetStringLibrary.Concat_StrStr` "Attack Speed and Damage Bonus for: " (`KismetStringLibrary.Conv_IntToString` (`self.Upgrade Cost`)) " Coins"))))
    (:`NewEnumerator2`
      (`TextRenderComponent.K2_SetText` (`self.TextRender`) (`KismetTextLibrary.Conv_StringToText` (`KismetStringLibrary.Concat_StrStr` "Increase blocking movement speed for: " (`KismetStringLibrary.Conv_IntToString` (`self.Upgrade Cost`)) " Coins"))))))

(event `self.ReceiveTick`
  (params (DeltaSeconds :type "Float (single-precision)"))
  (`SceneComponent.K2_SetWorldRotation` (`self.TextRender`) (`KismetMathLibrary.FindLookAtRotation` (`SceneComponent.K2_GetComponentLocation` (`self.TextRender`)) (`SceneComponent.K2_GetComponentLocation` (`PlayerCameraManager.TransformComponent` (`GameplayStatics.GetPlayerCameraManager` 0)))) false false))

(event `ResetNode`
  (bind _upgrade_cost (`self.Upgrade Cost`))
  (`SceneComponent.SetVisibility` (`self.TextRender`) true false)
  (`SceneComponent.SetVisibility` (`self.Collectible`) true false)
  (goto _label :!via `Reset`))

(event `self.Capsule.OnComponentBeginOverlap`
  (params (OverlappedComponent :type "PrimitiveComponent Object Reference") (OtherActor :type "Actor Object Reference") (OtherComp :type "PrimitiveComponent Object Reference") (OtherBodyIndex :type Integer) (bFromSweep :type Boolean) (SweepResult :type "HitResult Structure (by ref)"))
  (bind _upgrade_cost (`self.Upgrade Cost`))
  (`/Engine/EditorBlueprintResources/StandardMacros.DoOnce` false :!label _label
    (:`Completed`
      (bind _asbp_third_person_character (cast `/Game/ThirdPerson/Blueprints/BP_ThirdPersonCharacter` OtherActor)
        (:`then`
          (bind _currentcoinsamount (`/Game/ThirdPerson/Blueprints/BP_ThirdPersonCharacter.CurrentCoinsAmount` _asbp_third_person_character))
          (if (>= _currentcoinsamount _upgrade_cost)
            (set `/Game/ThirdPerson/Blueprints/BP_ThirdPersonCharacter.CurrentCoinsAmount` (- _currentcoinsamount _upgrade_cost) _asbp_third_person_character)
            (message `/Game/Blueprints/BPI_Player.UpgradePlayer` _asbp_third_person_character (`self.Type`))
            (`SceneComponent.SetVisibility` (`self.TextRender`) false false)
            (`SceneComponent.SetVisibility` (`self.Collectible`) false false)
            (`KismetSystemLibrary.Delay` 3.0)
            (`self.ResetNode`)
            (else
              (`self.ResetNode` :!label _label_2))))
        (:`CastFailed`
          (goto _label_2))))))

(fn `UserConstructionScript`
  (`parent.UserConstructionScript`))
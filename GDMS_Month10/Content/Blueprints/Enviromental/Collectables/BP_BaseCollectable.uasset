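; BP_BaseCollectable is a pickup actor that flies toward the third-person player character and destroys itself when collected.
; Actor overlap plays a movement sound and starts a timeline that lerps the actor from its current location to the player's live location each update, creating a homing pull.
; Overlap on the Collectable component plays the pickup sound, stops the timeline and destroys the actor.
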(event `self.ReceiveActorBeginOverlap`
  (params (OtherActor :type "Actor Object Reference"))
  (if (== (`GameplayStatics.GetObjectClass` OtherActor) "/Game/ThirdPerson/Blueprints/BP_ThirdPersonCharacter.BP_ThirdPersonCharacter_C")
    (`GameplayStatics.PlaySound2D` (`self.MovementSound`) 1.0 1.0 0.0 null null)
    (bind (_direction _alpha) (`Timeline|TL_Animation` :!via `PlayFromStart`)
      (:`Update`
        (`self.K2_SetActorLocation` (`KismetMathLibrary.VLerp` (`self.K2_GetActorLocation`) (`self.K2_GetActorLocation` OtherActor) _alpha))))))

(event `self.Collectable.OnComponentBeginOverlap`
  (params (OverlappedComponent :type "PrimitiveComponent Object Reference") (OtherActor :type "Actor Object Reference") (OtherComp :type "PrimitiveComponent Object Reference") (OtherBodyIndex :type Integer) (bFromSweep :type Boolean) (SweepResult :type "HitResult Structure (by ref)"))
  (if (== (`GameplayStatics.GetObjectClass` OtherActor) "/Game/ThirdPerson/Blueprints/BP_ThirdPersonCharacter.BP_ThirdPersonCharacter_C")
    (`GameplayStatics.PlaySound2D` (`self.PickupSound`) 1.0 1.0 0.0 null null)
    (`TimelineComponent.Stop` (`self.TL_Animation`))
    (`self.K2_DestroyActor`)))

(fn `UserConstructionScript`)
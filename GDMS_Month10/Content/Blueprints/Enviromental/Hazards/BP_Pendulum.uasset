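; Swinging pendulum hazard that damages actors it hits and knocks back the player character.
; After a configurable delay, a timeline swings the pivot through a 180-degree arc, reversing endlessly at each end with a whoosh sound.
; Collision overlap sends a damage message to any actor, then launches BP_ThirdPersonCharacter along the direction from the collision to the actor origin, with added upward lift.
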(event `self.ReceiveBeginPlay`
  (`KismetSystemLibrary.Delay` (`self.Delay`))
  (`self.Forward`))

(event `Forward`
  (`GameplayStatics.PlaySoundAtLocation` "/Game/SFX/Enviromental/Whoosh.Whoosh" (`self.K2_GetActorLocation`) (struct) 1.0 1.0 0.0 null null null null)
  (bind (_direction _alpha) (`Timeline|Movement Timeline` :!label _label)
    (:`Update`
      (`SceneComponent.K2_SetRelativeRotation` (`self.Pivot`) (`KismetMathLibrary.RLerp` (struct :`Pitch` 90.0) (struct :`Pitch` -90.0) _alpha) false false))
    (:`Finished`
      (if (`|EnumEquality` _direction "Forward")
        (`self.Reverse`)
        (else
          (`self.Forward`))))))

(event `Reverse`
  (`GameplayStatics.PlaySoundAtLocation` "/Game/SFX/Enviromental/Whoosh.Whoosh" (`self.K2_GetActorLocation`) (struct) 1.0 1.0 0.0 null null null null)
  (goto _label :!via `Reverse`))

(event `self.Collision.OnComponentBeginOverlap`
  (params (OverlappedComponent :type "PrimitiveComponent Object Reference") (OtherActor :type "Actor Object Reference") (OtherComp :type "PrimitiveComponent Object Reference") (OtherBodyIndex :type Integer) (bFromSweep :type Boolean) (SweepResult :type "HitResult Structure (by ref)"))
  (message `/Game/Blueprints/BPI_Damage.Take Damage` OtherActor 1 self)
  (bind _asbp_third_person_character (cast `/Game/ThirdPerson/Blueprints/BP_ThirdPersonCharacter` OtherActor))
  (`Character.LaunchCharacter` _asbp_third_person_character (+ (* (`KismetMathLibrary.Normal` (- (`self.K2_GetActorLocation`) (`SceneComponent.K2_GetComponentLocation` (`self.Collision`)))) 3000.0) (* (`self.GetActorUpVector`) 150.0)) false false))

(fn `UserConstructionScript`)
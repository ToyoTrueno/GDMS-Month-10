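; Spike trap hazard that repeatedly shoots up and retracts after a starting delay, with configurable travel and wait times.
; One timeline lerps Spike2 between down and up locations, with play rate set from the rise or lower time.
; A FlipFlop on timeline completion alternates the hold delays and reverses direction to sustain the loop.
; DamageTrigger overlaps send a TakeDamage message to the other actor, with no spike-state check.
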(event `self.ReceiveBeginPlay`
  (`KismetSystemLibrary.Delay` (`self.StartingDelay`))
  (`self.ShootUp`))

(event `ShootUp`
  (`TimelineComponent.SetPlayRate` (`self.TL_SpikeMovement`) (/ 1.0 (`self.RiseTime`)))
  (bind (_direction _alpha) (`Timeline|TL_SpikeMovement` :!via `PlayFromStart` :!label _label)
    (:`Update`
      (`SceneComponent.K2_SetRelativeLocation` (`self.Spike2`) (`KismetMathLibrary.VLerp` (`self.DownLocation`) (`self.UpLocation`) _alpha) false false))
    (:`Finished`
      (`/Engine/EditorBlueprintResources/StandardMacros.FlipFlop`
        (:`A`
          (`KismetSystemLibrary.Delay` (`self.LengthToStayUp`))
          (`self.RetractDown`))
        (:`B`
          (`KismetSystemLibrary.Delay` (`self.LengthToStayDown`))
          (`self.ShootUp`))))))

(event `RetractDown`
  (`TimelineComponent.SetPlayRate` (`self.TL_SpikeMovement`) (/ 1.0 (`self.LowerTime`)))
  (goto _label :!via `ReverseFromEnd`))

(event `self.DamageTrigger.OnComponentBeginOverlap`
  (params (OverlappedComponent :type "PrimitiveComponent Object Reference") (OtherActor :type "Actor Object Reference") (OtherComp :type "PrimitiveComponent Object Reference") (OtherBodyIndex :type Integer) (bFromSweep :type Boolean) (SweepResult :type "HitResult Structure (by ref)"))
  (message `/Game/Blueprints/BPI_Damage.Take Damage` OtherActor (`self.DamageAmount`) null))

(fn `UserConstructionScript`)
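; Trap door hazard that swings open once when the player steps into its trigger box.
; An overlap from any actor implementing BPI_Player passes a DoOnce, plays a door slam sound, then calls Trigger after a brief delay.
; Trigger plays a timeline that rotates two pivots in opposite directions to a quarter turn, with play rate scaled by TimeToOpen on BeginPlay.
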(event `self.ReceiveBeginPlay`
  (`TimelineComponent.SetPlayRate` (`self.OpenTrapDoorTimeline`) (/ 1.0 (`self.TimeToOpen`))))

(event `self.Box.OnComponentBeginOverlap`
  (params (OverlappedComponent :type "PrimitiveComponent Object Reference") (OtherActor :type "Actor Object Reference") (OtherComp :type "PrimitiveComponent Object Reference") (OtherBodyIndex :type Integer) (bFromSweep :type Boolean) (SweepResult :type "HitResult Structure (by ref)"))
  (if (`KismetSystemLibrary.DoesImplementInterface` OtherActor "/Game/Blueprints/BPI_Player.BPI_Player_C")
    (`/Engine/EditorBlueprintResources/StandardMacros.DoOnce` false
      (:`Completed`
        (`GameplayStatics.PlaySoundAtLocation` "/Game/SFX/Enviromental/door-slam-172171.door-slam-172171" (`self.K2_GetActorLocation`) (struct) 1.0 1.0 0.0 null null null null)
        (`KismetSystemLibrary.Delay` 0.1)
        (`/Game/Interfaces/BPI_Trigger.Trigger`)))))

(event `/Game/Interfaces/BPI_Trigger.Trigger`
  (bind (_direction _alpha) (`Timeline|OpenTrapDoorTimeline`)
    (:`Update`
      (`SceneComponent.K2_SetRelativeRotation` (`self.Pivot`) (`KismetMathLibrary.RLerp` (struct) (struct :`Pitch` 90.0) _alpha) false false)
      (`SceneComponent.K2_SetRelativeRotation` (`self.Pivot1`) (`KismetMathLibrary.RLerp` (struct) (struct :`Pitch` -90.0) _alpha) false false))))

(fn `UserConstructionScript`)
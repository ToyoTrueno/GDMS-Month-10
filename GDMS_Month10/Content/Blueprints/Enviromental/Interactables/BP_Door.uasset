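; BP_Door is an interactable door that moves between a closed start transform and an authored end transform.
; A timeline, rate-scaled by TimeToReachEnd, lerps the whole actor transform without sweep.
; Interact plays it forward or in reverse based on AtEnd, which a FlipFlop toggles on completion.
; The start is captured at BeginPlay, while the construction script records the end whenever SetEndTransform is ticked, then clears that flag.
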(event `self.ReceiveBeginPlay`
  (set `self.StartTransform` (`self.GetTransform`))
  (`TimelineComponent.SetPlayRate` (`self.TL_DoorOpen/Close`) (/ 1.0 (`self.TimeToReachEnd`))))

(event `/Game/Interfaces/BPI_Interact.Interact`
  (if (not (`self.AtEnd?`))
    (bind (_direction _alpha) (`Timeline|TL_DoorOpen/Close` :!via `PlayFromStart` :!label _label)
      (:`Update`
        (`self.K2_SetActorTransform` (`KismetMathLibrary.TLerp` (`self.StartTransform`) (`self.EndTransform`) _alpha)))
      (:`Finished`
        (bind _isa (`/Engine/EditorBlueprintResources/StandardMacros.FlipFlop`)
          (:`A`
            _)
          (:`B`
            _))
        (set `self.AtEnd?` _isa)))
    (else
      (goto _label :!via `ReverseFromEnd`))))

(fn `UserConstructionScript`
  (if (`self.SetEndTransform`)
    (set `self.EndTransform` (`self.GetTransform`))
    (set `self.SetEndTransform` false)))
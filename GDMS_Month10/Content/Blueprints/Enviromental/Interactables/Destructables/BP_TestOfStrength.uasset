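; BP_TestOfStrength is a destructible interactable that breaks only when one hit deals exactly the required damage, and otherwise plays a failure sound.
; On the first qualifying hit, a DoOnce gate lets it play a sound, swap its static mesh for a newly added geometry collection and spawn a burst of pickups flagged as coming from a breakable.
; The actor destroys itself after a short delay.
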(event `/Game/Blueprints/BPI_Damage.Take Damage`
  (params (IncomingDamage :type Integer) (Source :type "Actor Object Reference"))
  (if (== IncomingDamage (`self.DamageRequired`))
    (`/Engine/EditorBlueprintResources/StandardMacros.DoOnce` false
      (:`Completed`
        (`GameplayStatics.PlaySound2D` "/Engine/VREditor/Sounds/UI/Drop_Item_From_ContentBrowser.Drop_Item_From_ContentBrowser" 1.0 1.0 0.0 null null)
        (`ActorComponent.K2_DestroyComponent` (`self.StaticMesh`))
        (`AddComponent|NODE_AddGeometryCollectionComponent-0`)
        (for _ (range 51)
          (`|SpawnActorFromClass` (`self.PickupToSpawn`) (`self.GetTransform`) "AlwaysSpawn" "MultiplyWithRoot" null true null))
        (`KismetSystemLibrary.Delay` 5.0)
        (`self.K2_DestroyActor`)))
    (else
      (`GameplayStatics.PlaySound2D` "/Engine/EditorSounds/Notifications/CompileFailed.CompileFailed" 1.0 1.0 0.0 null null))))

(fn `UserConstructionScript`)
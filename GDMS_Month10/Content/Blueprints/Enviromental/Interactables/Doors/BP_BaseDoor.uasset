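; Base interactable door that moves between its starting relative transform and a configurable offset over a set time.
; Trigger plays or reverses a timeline that lerps the door transform, using a FlipFlop to track direction and allow mid-motion reversal.
; An optional camera pan messages the player character and waits out the blend first.
; The construction script removes unused camera and proximity components; Trigger does nothing when TriggerWhenNear is set.
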(event `self.ReceiveBeginPlay`
  (bind (_relativemovement_location _relativemovement_rotation) (`KismetMathLibrary.BreakTransform` (`self.RelativeMovement`)))
  (bind _output_get (set `self.StartTransform` (`SceneComponent.GetRelativeTransform` (`self.Door`))))
  (set `self.EndTransform` (`KismetMathLibrary.MakeTransform` (+ (.location _output_get) _relativemovement_location) (`KismetMathLibrary.ComposeRotators` (.rotation _output_get) _relativemovement_rotation) (.scale _output_get)))
  (`TimelineComponent.SetPlayRate` (`self.TL_DoorOpen/Close`) (/ 1.0 (`self.TimeToReachEnd`))))

(event `/Game/Interfaces/BPI_Trigger.Trigger`
  (bind _tl_dooropen_close (`self.TL_DoorOpen/Close`))
  (if (not (`self.TriggerWhenNear`))
    (if (`self.PanCamera`)
      (message `/Game/Blueprints/BPI_Player.PanCamera` (`GameplayStatics.GetPlayerCharacter` 0) self (`self.CameraBlendTime`))
      (`KismetSystemLibrary.Delay` (`self.CameraBlendTime`)))
    (if (`TimelineComponent.IsPlaying` _tl_dooropen_close)
      (`TimelineComponent.Stop` _tl_dooropen_close)
      (`|ExecutionSequence`
        (:`then_0`
          (bind _isa (`/Engine/EditorBlueprintResources/StandardMacros.FlipFlop` :!label _label)
            (:`A`
              _)
            (:`B`
              _))
          (set `self.AtEnd?` _isa))
        (:`then_1`
          (if (not (`self.AtEnd?`)) :!label _label_2
            (bind (_direction _alpha) (`Timeline|TL_DoorOpen/Close` :!label _label_3)
              (:`Update`
                (`SceneComponent.K2_SetRelativeTransform` (`self.Door`) (`KismetMathLibrary.TLerp` (`self.StartTransform`) (`self.EndTransform`) _alpha) false false))
              (:`Finished`
                (goto _label)))
            (else
              (goto _label_3 :!via `Reverse`)))))
      (else
        (goto _label_2)))))

(fn `UserConstructionScript`
  (if (not (`self.TriggerWhenNear`))
    (`ActorComponent.K2_DestroyComponent` (`self.NearbyCollision`)))
  (if (not (`self.PanCamera`))
    (`ActorComponent.K2_DestroyComponent` (`self.Camera`))))
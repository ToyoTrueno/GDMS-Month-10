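; Base pivot door that swings open when the third-person character comes near and closes when they leave, if TriggerWhenNear is set.
; On overlap, the dot product of the door's forward vector and the direction to the character picks the side of the 90-degree swing.
; A timeline interpolates the door's relative rotation toward that target and reverses on exit, with its play rate derived from TimeToReachEnd.
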(event `self.ReceiveBeginPlay`
  (`parent.ReceiveBeginPlay`)
  (if (`self.TriggerWhenNear`)
    (set `self.StartTransform` (`KismetMathLibrary.MakeTransform` (0.0 0.0 0.0)))
    (`TimelineComponent.SetPlayRate` (`self.TL_NearDoorAnimation`) (/ 1.0 (`self.TimeToReachEnd`)))))

(event `Open Door`
  (bind (_direction _alpha) (`Timeline|TL_NearDoorAnimation` :!label _label)
    (:`Update`
      (bind (_returnvalue_location _returnvalue_rotation) (`KismetMathLibrary.BreakTransform` (`KismetMathLibrary.TLerp` (`self.StartTransform`) (`self.EndTransform`) _alpha)))
      (`SceneComponent.K2_SetRelativeTransform` (`self.Door`) (`KismetMathLibrary.MakeTransform` (0.0 0.0 0.0) _returnvalue_rotation) false false))))

(event `Close Door`
  (goto _label :!via `Reverse`))

(event `self.NearbyCollision.OnComponentBeginOverlap`
  (params (OverlappedComponent :type "PrimitiveComponent Object Reference") (OtherActor :type "Actor Object Reference") (OtherComp :type "PrimitiveComponent Object Reference") (OtherBodyIndex :type Integer) (bFromSweep :type Boolean) (SweepResult :type "HitResult Structure (by ref)"))
  (if (and (`self.TriggerWhenNear`) (== (`GameplayStatics.GetObjectClass` OtherActor) "/Game/ThirdPerson/Blueprints/BP_ThirdPersonCharacter.BP_ThirdPersonCharacter_C"))
    (`self.Set Rotation` OtherActor)
    (`self.Open Door`)))

(event `self.NearbyCollision.OnComponentEndOverlap`
  (params (OverlappedComponent :type "PrimitiveComponent Object Reference") (OtherActor :type "Actor Object Reference") (OtherComp :type "PrimitiveComponent Object Reference") (OtherBodyIndex :type Integer))
  (if (and (`self.TriggerWhenNear`) (== (`GameplayStatics.GetObjectClass` OtherActor) "/Game/ThirdPerson/Blueprints/BP_ThirdPersonCharacter.BP_ThirdPersonCharacter_C"))
    (`self.Close Door`)))

(fn `Set Rotation`
  (params (self2 :type "Actor Object Reference"))
  (bind _output_get (set `self.HalfSpaceValue` (`KismetMathLibrary.Dot_VectorVector` (`KismetMathLibrary.Normal` (- (`self.K2_GetActorLocation` self2) (`SceneComponent.K2_GetComponentLocation` (`self.Door`)))) (`SceneComponent.GetForwardVector` (`self.Door`)))))
  (set `self.EndTransform` (`KismetMathLibrary.MakeTransform` (0.0 0.0 0.0) (`KismetMathLibrary.ComposeRotators` (`SceneComponent.RelativeRotation` (`self.Door`)) (select `bool` (>= _output_get 0.0) :`false` (struct :`Yaw` 90.0) :`true` (struct :`Yaw` -90.0) :!type "Rotator Structure")))))

(fn `UserConstructionScript`
  (`parent.UserConstructionScript`))
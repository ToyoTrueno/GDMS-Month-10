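; Base sliding door interactable that moves its Door component between a start and end transform.
; A timeline lerps the relative transform, played by the OpenDoor event and reversed by CloseDoor.
; With TriggerWhenNear set, Box overlaps by BP_ThirdPersonCharacter open and close it automatically, and BeginPlay scales the timeline rate from TimeToReachEnd.
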(event `self.ReceiveBeginPlay`
  (`parent.ReceiveBeginPlay`)
  (if (`self.TriggerWhenNear`)
    (`TimelineComponent.SetPlayRate` (`self.TL_NearDoorAnimation`) (/ 1.0 (`self.TimeToReachEnd`)))))

(event `Open Door`
  (bind (_direction _alpha) (`Timeline|TL_NearDoorAnimation` :!label _label)
    (:`Update`
      (`SceneComponent.K2_SetRelativeTransform` (`self.Door`) (`KismetMathLibrary.TLerp` (`self.StartTransform`) (`self.EndTransform`) _alpha) false false))))

(event `Close Door`
  (goto _label :!via `Reverse`))

(event `self.Box.OnComponentBeginOverlap`
  (params (OverlappedComponent :type "PrimitiveComponent Object Reference") (OtherActor :type "Actor Object Reference") (OtherComp :type "PrimitiveComponent Object Reference") (OtherBodyIndex :type Integer) (bFromSweep :type Boolean) (SweepResult :type "HitResult Structure (by ref)"))
  (if (and (`self.TriggerWhenNear`) (== (`GameplayStatics.GetObjectClass` OtherActor) "/Game/ThirdPerson/Blueprints/BP_ThirdPersonCharacter.BP_ThirdPersonCharacter_C"))
    (`self.Open Door`)))

(event `self.Box.OnComponentEndOverlap`
  (params (OverlappedComponent :type "PrimitiveComponent Object Reference") (OtherActor :type "Actor Object Reference") (OtherComp :type "PrimitiveComponent Object Reference") (OtherBodyIndex :type Integer))
  (if (and (`self.TriggerWhenNear`) (== (`GameplayStatics.GetObjectClass` OtherActor) "/Game/ThirdPerson/Blueprints/BP_ThirdPersonCharacter.BP_ThirdPersonCharacter_C"))
    (`self.Close Door`)
    (`self.Close Door`)))

(fn `UserConstructionScript`
  (`parent.UserConstructionScript`))
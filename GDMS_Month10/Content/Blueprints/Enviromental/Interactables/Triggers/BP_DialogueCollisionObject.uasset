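; BP_DialogueCollisionObject is a trigger that shows a dialogue message on screen when the third-person character overlaps it.
; It writes its main and small text into the character's GameMessage widget and can stop firing once an optional countdown runs out.
; After a delay it removes the message only if the player's current text still matches its own.
; An optional setting also removes it when the character leaves.
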(event `self.ReceiveActorBeginOverlap`
  (params (OtherActor :type "Actor Object Reference"))
  (bind _asbp_third_person_character (cast `/Game/ThirdPerson/Blueprints/BP_ThirdPersonCharacter` OtherActor))
  (if (not (`self.Done`))
    (set `/Game/ThirdPerson/Blueprints/BP_ThirdPersonCharacter.GameMessageText` (`self.Dialogue Text`) _asbp_third_person_character)
    (set `/Game/ThirdPerson/Blueprints/BP_ThirdPersonCharacter.SmallText` (`self.SmallText`) _asbp_third_person_character)
    (bind _gamemessage (`/Game/ThirdPerson/Blueprints/BP_ThirdPersonCharacter.GameMessage` _asbp_third_person_character))
    (`/Game/Blueprints/WBP_GameMessage.Change Text` _gamemessage)
    (`UserWidget.AddToViewport` _gamemessage 0)
    (if (`self.DoUntil`)
      (if (<= (`self.CountUntilDone`) 0)
        (set `self.Done` true)
        (else
          (set `self.CountUntilDone` (- (`self.CountUntilDone`) 1)))))
    (`KismetSystemLibrary.Delay` (`self.DisappearAfter`))
    (bind _asbp_third_person_character_2 (cast `/Game/ThirdPerson/Blueprints/BP_ThirdPersonCharacter` (`GameplayStatics.GetPlayerCharacter` 0)))
    (if (`KismetTextLibrary.EqualEqual_TextText` (`self.Dialogue Text`) (`/Game/ThirdPerson/Blueprints/BP_ThirdPersonCharacter.GameMessageText` _asbp_third_person_character_2))
      (`Widget.RemoveFromParent` _gamemessage))))

(event `self.ReceiveActorEndOverlap`
  (params (OtherActor :type "Actor Object Reference"))
  (bind _asbp_third_person_character (cast `/Game/ThirdPerson/Blueprints/BP_ThirdPersonCharacter` OtherActor))
  (if (`self.OnCollisionLeave`)
    (`Widget.RemoveFromParent` (`/Game/ThirdPerson/Blueprints/BP_ThirdPersonCharacter.GameMessage` _asbp_third_person_character))))

(fn `UserConstructionScript`)
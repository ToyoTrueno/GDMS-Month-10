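; BP_CastleEntranceDoor is a castle entrance door puzzle gated by five collectible crests on a podium.
; PickUpItem flags each collected item by index in the PickedUp array.
; Interacting with the Podium reveals the matching crest components, registered in the construction script, then checks that all are visible.
; Once every crest shows, a DoOnce calls Trigger a single time.
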(event `/Game/Blueprints/BPI_ItemPickUp.Pick Up Item`
  (params (Pickup :type String))
  (`KismetArrayLibrary.Array_Set` (`self.PickedUp`) (`KismetStringLibrary.Conv_StringToInt` Pickup) true))

(event `self.Interact`
  (params (HitComponent :type "ActorComponent Object Reference"))
  (if (== HitComponent (`self.Podium`))
    (for (_array_element _array_index) (`self.PickedUp`)
      (if _array_element
        (`SceneComponent.SetVisibility` (`|GetArrayItem` (`self.Crests`) _array_index) true false)))
    (set `self.AllCollected` true)
    (for _array_element_2 (`self.Crests`)
      (if (not (`SceneComponent.IsVisible` _array_element_2))
        (set `self.AllCollected` false)))
    (if (`self.AllCollected`)
      (`/Engine/EditorBlueprintResources/StandardMacros.DoOnce` false
        (:`Completed`
          (`self.Trigger`))))))

(fn `UserConstructionScript`
  (bind _crests (`self.Crests`))
  (`parent.UserConstructionScript`)
  (`KismetArrayLibrary.Array_Add` _crests (`self.PodiumCrest 1`))
  (`KismetArrayLibrary.Array_Add` _crests (`self.PodiumCrest 2`))
  (`KismetArrayLibrary.Array_Add` _crests (`self.PodiumCrest 3`))
  (`KismetArrayLibrary.Array_Add` _crests (`self.PodiumCrest 4`))
  (`KismetArrayLibrary.Array_Add` _crests (`self.PodiumCrest 5`)))
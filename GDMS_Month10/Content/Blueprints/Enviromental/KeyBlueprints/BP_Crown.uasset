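; BP_Crown is an interactable crown that triggers the boss once all four of its gems are in place.
; PickUpItem flags collected pickups by index, and Interact reveals the matching gem components gathered in the Construction Script.
; When every gem is visible, it fires TriggerBoss once, plays a scared sound and removes its prompt.
; The PressE overlap shows that text prompt only for actors implementing BPI_Player.
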(event `self.ReceiveBeginPlay`
  (`SceneComponent.SetVisibility` (`self.TextRender`) false false))

(event `/Game/Blueprints/BPI_ItemPickUp.Pick Up Item`
  (params (Pickup :type String))
  (`KismetArrayLibrary.Array_Set` (`self.PickedUp`) (`KismetStringLibrary.Conv_StringToInt` Pickup) true))

(event `/Game/Interfaces/BPI_Trigger.Interact`
  (params (HitComponent :type "ActorComponent Object Reference"))
  (for (_array_element _array_index) (`self.PickedUp`)
    (if _array_element
      (`SceneComponent.SetVisibility` (`|GetArrayItem` (`self.Gems`) _array_index) true false)))
  (set `self.AllCollected` true)
  (for _array_element_2 (`self.Gems`)
    (if (not (`SceneComponent.IsVisible` _array_element_2))
      (set `self.AllCollected` false)))
  (if (`self.AllCollected`)
    (`/Engine/EditorBlueprintResources/StandardMacros.DoOnce` false
      (:`Completed`
        (`self.TriggerBoss`)
        (`GameplayStatics.PlaySound2D` "/Game/SFX/GobSounds/Emotion/Scared/Gob_Emotion_Scared.Gob_Emotion_Scared" 1.0 1.0 0.0 null null)
        (`ActorComponent.K2_DestroyComponent` (`self.Press "E"`))
        (`ActorComponent.K2_DestroyComponent` (`self.TextRender`))))))

(event `self.Press "E".OnComponentBeginOverlap`
  (params (OverlappedComponent :type "PrimitiveComponent Object Reference") (OtherActor :type "Actor Object Reference") (OtherComp :type "PrimitiveComponent Object Reference") (OtherBodyIndex :type Integer) (bFromSweep :type Boolean) (SweepResult :type "HitResult Structure (by ref)"))
  (if (`KismetSystemLibrary.DoesImplementInterface` OtherActor "/Game/Blueprints/BPI_Player.BPI_Player_C")
    (`SceneComponent.SetVisibility` (`self.TextRender`) true false)))

(event `self.Press "E".OnComponentEndOverlap`
  (params (OverlappedComponent :type "PrimitiveComponent Object Reference") (OtherActor :type "Actor Object Reference") (OtherComp :type "PrimitiveComponent Object Reference") (OtherBodyIndex :type Integer))
  (if (`KismetSystemLibrary.DoesImplementInterface` OtherActor "/Game/Blueprints/BPI_Player.BPI_Player_C")
    (`SceneComponent.SetVisibility` (`self.TextRender`) false false)))

(fn `UserConstructionScript`
  (bind _gems (`self.Gems`))
  (`KismetArrayLibrary.Array_Add` _gems (`self.GemPlacement1`))
  (`KismetArrayLibrary.Array_Add` _gems (`self.GemPlacement2`))
  (`KismetArrayLibrary.Array_Add` _gems (`self.GemPlacement3`))
  (`KismetArrayLibrary.Array_Add` _gems (`self.GemPlacement4`)))
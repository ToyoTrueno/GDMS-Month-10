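; Windmill environment actor that rotates through a RotatingMovement component and carries four platform child actors.
; On BeginPlay it applies its RotationRate variable to a single axis of that movement component.
; It then sends the same rate to each platform through a SetRotationRateMessage call, so the windmill and platforms share one speed value.
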(event `self.ReceiveBeginPlay`
  (set `RotatingMovementComponent.RotationRate` (`KismetMathLibrary.MakeRotator` (`self.RotationRate`)) (`self.RotatingMovement`))
  (for _index (range 4)
    (message `/Game/Interfaces/BPI_Trigger.SetRotationRate` (select `int` _index :`0` (`ChildActorComponent.ChildActor` (`self.BP_WindmillPlatform3`)) :`1` (`ChildActorComponent.ChildActor` (`self.BP_WindmillPlatform1`)) :`2` (`ChildActorComponent.ChildActor` (`self.BP_WindmillPlatform2`)) :`3` (`ChildActorComponent.ChildActor` (`self.BP_WindmillPlatform`)) :!type "Object Object Reference") (`self.RotationRate`))))

(fn `UserConstructionScript`)
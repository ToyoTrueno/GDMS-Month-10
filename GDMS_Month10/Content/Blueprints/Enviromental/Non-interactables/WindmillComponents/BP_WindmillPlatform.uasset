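; Windmill platform component that gently rocks back and forth and can spin at an externally set rate.
; After a random start delay, a Timeline tilts the Pivot between two opposite angles, alternating forward and reverse endlessly.
; SetRotationRate applies the negated input rate to a single axis of RotatingMovement, apparently to counter the windmill's rotation.
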(event `self.ReceiveBeginPlay`
  (`KismetSystemLibrary.Delay` (`KismetMathLibrary.RandomFloatInRange` 0.0 1.0))
  (`self.Forward`))

(event `Forward`
  (bind (_direction _alpha) (`Timeline|Timeline` :!label _label)
    (:`Update`
      (`SceneComponent.K2_SetRelativeRotation` (`self.Pivot`) (`KismetMathLibrary.RLerp` (struct :`Roll` 5.0) (struct :`Roll` -5.0) _alpha) false false))
    (:`Finished`
      (if (`|EnumEquality` _direction "Forward")
        (`self.Reverse`)
        (else
          (`self.Forward`))))))

(event `Reverse`
  (goto _label :!via `Reverse`))

(event `/Game/Interfaces/BPI_Trigger.SetRotationRate`
  (params (Rate :type "Float (double-precision)"))
  (set `RotatingMovementComponent.RotationRate` (`KismetMathLibrary.MakeRotator` (* Rate -1.0)) (`self.RotatingMovement`)))

(fn `UserConstructionScript`)
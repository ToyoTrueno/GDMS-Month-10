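; Base pickup actor that, when the third-person character overlaps it, flies to the player and is collected.
; Box collision starts disabled and becomes query-only shortly after BeginPlay.
; A one-time overlap plays a sound and runs a timeline lerping the actor toward just below the player's location.
; On finish it plays the pickup sound, sends PickUpItemMessage with its Item to the player and parent actor, then destroys itself.
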(event `self.ReceiveBeginPlay`
  (`PrimitiveComponent.SetCollisionEnabled` (`self.Box`) "NoCollision")
  (`KismetSystemLibrary.Delay` 0.25)
  (`PrimitiveComponent.SetCollisionEnabled` (`self.Box`) "QueryOnly"))

(event `self.ReceiveActorBeginOverlap`
  (params (OtherActor :type "Actor Object Reference"))
  (if (== (`GameplayStatics.GetObjectClass` OtherActor) "/Game/ThirdPerson/Blueprints/BP_ThirdPersonCharacter.BP_ThirdPersonCharacter_C")
    (`/Engine/EditorBlueprintResources/StandardMacros.DoOnce` false
      (:`Completed`
        (set `self.Player` OtherActor)
        (`GameplayStatics.PlaySound2D` (`self.MovementSound`) 1.0 1.0 0.0 null null)
        (bind (_direction _alpha) (`Timeline|TL_Animation` :!via `PlayFromStart`)
          (:`Update`
            (`self.K2_SetActorLocation` (`KismetMathLibrary.VLerp` (`self.K2_GetActorLocation`) (- (`self.K2_GetActorLocation` (`self.Player`)) (0.0 0.0 25.0)) _alpha)))
          (:`Finished`
            (`/Engine/EditorBlueprintResources/StandardMacros.DoOnce` false
              (:`Completed`
                (`GameplayStatics.PlaySound2D` (`self.PickupSound`) 1.0 1.0 0.0 null null)
                (message `/Game/Blueprints/BPI_ItemPickUp.Pick Up Item` (`self.Player`) (`self.Item`))
                (message `/Game/Blueprints/BPI_ItemPickUp.Pick Up Item` (`self.GetParentActor`) (`self.Item`))
                (`self.K2_DestroyActor`)))))))))

(fn `UserConstructionScript`)
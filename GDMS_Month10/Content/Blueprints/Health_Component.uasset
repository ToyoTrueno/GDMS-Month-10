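; Health component that tracks hit points for its owning actor and handles incoming damage and death.
; CurHP starts at MaxHP on BeginPlay, and the TakeDamage event passes damage and its source to DamageLogic.
; DamageLogic checks CanTakeDamage, which currently always returns true, subtracts the damage, and calls DieMessage on the owner when HP is zero or below.
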(event `self.ReceiveBeginPlay`
  (set `self.CurHP` (`self.MaxHP`)))

(event `/Game/Blueprints/BPI_Damage.Take Damage`
  (params (IncomingDamage :type Byte) (Source :type "Actor Object Reference"))
  (`self.Damage Logic` IncomingDamage Source))

(fn `Can Take Damage`
  (params (Instigator :type "Actor Object Reference"))
  (returns (out :type Boolean))
  (return true))

(fn `Damage Logic`
  (params (InputPin :type Byte) (Instigator :type "Actor Object Reference"))
  (bind _out (`self.Can Take Damage` Instigator))
  (if _out
    (bind _output_get (set `self.CurHP` (- (`self.CurHP`) InputPin)))
    (if (<= _output_get 0)
      (message `/Game/Blueprints/BPI_Damage.Die` (`self.GetOwner`)))))
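; PlayerHP is the player's health component, extending a parent health class with shielding, healing and heart-based HUD feedback.
; ToggleInvuln flips IsShielded, which CanTakeDamage checks, while Heal adds to CurHP capped at MaxHP.
; TakeDamage feeds DamageLogic, which runs the parent logic and then messages the owner to damage hearts.
; AddHeartsToHUD sends the owner one add-HP message per whole point of MaxHP.
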(event `self.ReceiveBeginPlay`
  (`parent.ReceiveBeginPlay`))

(event `/Game/Blueprints/BPI_Player.Toggle Invuln`
  (set `self.IsShielded` (not (`self.IsShielded`))))

(event `/Game/Blueprints/BPI_Damage.Take Damage`
  (params (IncomingDamage :type Byte) (Source :type "Actor Object Reference"))
  (`self.Damage Logic` IncomingDamage Source))

(event `/Game/Blueprints/BPI_Damage.Heal`
  (params (`Heal Val` :type Byte))
  (bind _returnvalue (+ `Heal Val` (`self.CurHP`)))
  (if (> _returnvalue (`self.MaxHP`))
    (set `self.CurHP` (`self.MaxHP`))
    (else
      (set `self.CurHP` _returnvalue))))

(fn `Add Hearts to HUD`
  (locals (loopct :type Integer))
  (bind _output_get (set `local.loopct` (`KismetMathLibrary.Conv_ByteToInt` (`self.MaxHP`))))
  (while (> _output_get 0)
    (`/Engine/EditorBlueprintResources/StandardMacros.DecrementInt` (`local.loopct`)
      (:`  `
        (message `/Game/Interfaces/BPI_HUD.AddHP` (`self.GetOwner`))))))

(fn `Can Take Damage`
  (params (Instigator :type "Actor Object Reference"))
  (returns (out :type Boolean))
  (return (not (`self.IsShielded`))))

(fn `Damage Logic`
  (params (InputPin :type Byte) (Instigator :type "Actor Object Reference"))
  (`parent.Damage Logic` InputPin Instigator)
  (message `/Game/Interfaces/BPI_HUD.DamageHearts` (`self.GetOwner`)))
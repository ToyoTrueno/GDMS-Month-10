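; Arrow projectile fired by enemies that damages the player on contact.
; Each tick it rotates to face along its velocity so the arrow points where it flies.
; When its Box overlaps the player character, it spawns a hit Niagara effect, plays a skeleton arrow hit sound, sends a damage message to the player and destroys itself.
; Overlaps with anything other than the player are ignored.
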(event `self.ReceiveTick`
  (params (DeltaSeconds :type "Float (single-precision)"))
  (`self.K2_SetActorRotation` (`KismetMathLibrary.MakeRotFromX` (`KismetMathLibrary.Normal` (`self.GetVelocity`)))))

(event `self.Box.OnComponentBeginOverlap`
  (params (OverlappedComponent :type "PrimitiveComponent Object Reference") (OtherActor :type "Actor Object Reference") (OtherComp :type "PrimitiveComponent Object Reference") (OtherBodyIndex :type Integer) (bFromSweep :type Boolean) (SweepResult :type "HitResult Structure (by ref)"))
  (bind _returnvalue (`GameplayStatics.GetPlayerCharacter` 0))
  (if (== OtherActor _returnvalue)
    (`NiagaraFunctionLibrary.SpawnSystemAtLocation` "/Game/sA_Megapack_v1/sA_StylizedAttacksPack/FX/NiagaraSystems/NS_BasicHit_2.NS_BasicHit_2" (`self.K2_GetActorLocation`))
    (`GameplayStatics.PlaySound2D` "/Game/Characters/Enemies/EnemySounds/SkeletonArrowHit.SkeletonArrowHit" 10.0 1.0 0.0 null null)
    (message `/Game/Blueprints/BPI_Damage.Take Damage` _returnvalue 1 null)
    (`self.K2_DestroyActor`)))

(fn `UserConstructionScript`)
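; Base enemy Blueprint that holds state, idle type and wander/patrol data, exposed through getters and an UpdateState event.
; The construction script previews the idle setup with a wander sphere or numbered patrol-point labels.
; BeginPlay caches the sphere center before destroying it and converts patrol points from actor-relative offsets to world locations.
; Health component death destroys the actor, and DefaultAttack is a placeholder that prints and immediately reports finished.
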(event `self.ReceiveBeginPlay`
  (bind _wandersphere (`self.WanderSphere`))
  (bind _patrolpoints (`self.PatrolPoints`))
  ;[0.03955 0.4072 0.6584] Bind Death Event
  (add `/Game/BlueprintComponents/BPC_Health.Death` (`self.BPC_Health`) (`|CreateDelegate` :!event `Death`))
  ;[0.03955 0.4072 0.6584] Save Wander Center and Destroy it
  (set `self.WanderCenter` (`SceneComponent.K2_GetComponentLocation` _wandersphere))
  (`ActorComponent.K2_DestroyComponent` _wandersphere)
  ;[0.03955 0.4072 0.6584] Convert Patrol Points to World Location
  (for (_array_element _array_index) _patrolpoints
    (`KismetArrayLibrary.Array_Set` _patrolpoints _array_index (+ _array_element (`self.K2_GetActorLocation`)))))

(event `/Game/Interfaces/I_Enemy.DefaultAttack`
  ;[0.03955 0.4072 0.6584] Default Attack
  (`KismetSystemLibrary.PrintString` "Attack")
  (`self.FinishedAttack`))

(event `/Game/Interfaces/I_Enemy.UpdateState`
  (params (NewState :type "/Game/Characters/Enemies/Enums/E_EnemyStates Enum" :default "NewEnumerator0"))
  ;[0.03955 0.4072 0.6584] Change State Interface
  (`self.ChangeState` NewState))

(event `Death`
  ;[0.03955 0.4072 0.6584] Destroy Actor on Death
  (`self.K2_DestroyActor`))

(fn `ChangeState`
  (params (NewState :type "/Game/Characters/Enemies/Enums/E_EnemyStates Enum" :default "NewEnumerator0"))
  (set `self.State` NewState))

(fn `GetEnemyStates`
  (returns (EnemyState :type "/Game/Characters/Enemies/Enums/E_EnemyStates Enum") (IdleType :type "/Game/Characters/Enemies/Enums/E_IdleTypes Enum"))
  (return (`self.State`) (`self.IdleType`)))

(fn `GetPatrolPoints`
  (returns (PatrolPoints :type "Array of Vector Structure"))
  (return (`self.PatrolPoints`)))

(fn `GetWanderValues`
  (returns (Center :type "Vector Structure") (Radius :type "Float (double-precision)"))
  (return (`self.WanderCenter`) (`self.WanderSphereSize`)))

(fn `UserConstructionScript`
  (`|ExecutionSequence`
    (:`then_0`
      (`SceneComponent.SetVisibility` (`self.WanderSphere`) (`|EnumEquality` (`self.IdleType`) "NewEnumerator1") false)
      (`SphereComponent.SetSphereRadius` (`self.WanderSphere`) (`self.WanderSphereSize`) true)
      (`SceneComponent.K2_SetWorldLocation` (`self.WanderSphere`) (+ (`self.K2_GetActorLocation`) (`self.WanderSphereOffset`)) false false))
    (:`then_1`
      (for (_array_element _array_index) (`self.PatrolPoints`)
        (bind _returnvalue (`AddComponent|NODE_AddTextRenderComponent-0` :`RelativeTransform` (`KismetMathLibrary.MakeTransform` _array_element (struct) (2.0 2.0 2.0))))
        (`TextRenderComponent.K2_SetText` _returnvalue (`KismetSystemLibrary.MakeLiteralText` (`KismetTextLibrary.Conv_IntToText` (+ _array_index 1))))
        (`TextRenderComponent.SetTextRenderColor` _returnvalue (`KismetMathLibrary.Conv_LinearColorToColor` (struct :`R` 1.0 :`A` 1.0)))
        (`SceneComponent.SetVisibility` _returnvalue (`|EnumEquality` (`self.IdleType`) "NewEnumerator2") false)
        (`SceneComponent.SetHiddenInGame` _returnvalue true false)))))
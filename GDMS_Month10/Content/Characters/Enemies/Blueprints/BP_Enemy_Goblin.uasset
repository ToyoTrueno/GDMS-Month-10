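; Goblin enemy Blueprint that supplies the default melee attack against the player.
; DefaultAttack plays the goblin attack montage and calls FinishedAttack when it completes.
; On the montage's Attack notify, a debug-drawn sphere multi-trace at the right-hand socket sends TakeDamageMessage for hits matching the player character.
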(event `/Game/Interfaces/I_Enemy.DefaultAttack`
  (bind _returnvalue (`GameplayStatics.GetPlayerCharacter` 0))
  (bind _returnvalue_2 (`SceneComponent.GetSocketLocation` (`self.Mesh`) "hand_r"))
  (bind _notifyname (`|PlayMontage` (`self.Mesh`) "/Game/Characters/Enemies/Animations/Goblin/Enemy_Goblin_Attack_Montage.Enemy_Goblin_Attack_Montage")
    (:`OnCompleted`
      (`self.FinishedAttack`))
    (:`OnNotifyBegin`
      (switch `name` _notifyname
        (:`Attack`
          (bind _outhits (`KismetSystemLibrary.SphereTraceMulti` :`Start` _returnvalue_2 :`End` _returnvalue_2 :`Radius` 50.0 :`TraceChannel` "TraceTypeQuery1" :`DrawDebugType` "ForDuration"))
          (for _array_element _outhits
            (if (== (`.HitActor` (`GameplayStatics.BreakHitResult` _array_element)) _returnvalue)
              (message `/Game/Blueprints/BPI_Damage.Take Damage` _returnvalue 1 self))))))))

(fn `UserConstructionScript`
  (`parent.UserConstructionScript`))
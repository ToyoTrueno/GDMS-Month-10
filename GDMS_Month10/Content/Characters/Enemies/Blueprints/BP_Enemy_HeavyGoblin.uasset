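; Heavy goblin enemy with a charged melee attack that holds its wind-up until the player comes within reach.
; DefaultAttack plays a start montage into a slow, repeating loop, then arms a Tick distance check that triggers the end montage.
; That montage's Attack notify sphere-traces at the right palm to damage the player.
; Losing the player cancels the attack by toggling animation mode to reset montages, clearing AI focus and updating state.
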(event `self.DefaultAttack`
  (set `self.AttackMontageStarted` true)
  (`|PlayMontage` (`self.Mesh`) "/Game/Characters/Enemies/Animations/HeavyGoblin/HeavyGoblin_Attack_Start.HeavyGoblin_Attack_Start" 0.75
    (:`OnBlendOut`
      (`|ExecutionSequence`
        (:`then_0`
          (set `self.LoopAttackAnim` true)
          (`|PlayMontage` (`self.Mesh`) "/Game/Characters/Enemies/Animations/HeavyGoblin/HeavyGoblin_Attack_Loop.HeavyGoblin_Attack_Loop" 0.1 :!label _label
            (:`OnBlendOut`
              (if (`self.LoopAttackAnim`)
                (goto _label)))))
        (:`then_1`
          (`KismetSystemLibrary.Delay` 0.5)
          (set `self.ReadyToAttack` true))))))

(event `self.ReceiveTick`
  (params (DeltaSeconds :type "Float (single-precision)"))
  (bind _returnvalue (`GameplayStatics.GetPlayerCharacter` 0))
  (bind _returnvalue_2 (`SceneComponent.GetSocketLocation` (`self.Mesh`) "CATRigRArmPalm"))
  (if (`self.ReadyToAttack`)
    (if (<= (`KismetMathLibrary.VSize` (- (`self.K2_GetActorLocation` (`GameplayStatics.GetPlayerCharacter` 0)) (`self.K2_GetActorLocation`))) 200.0)
      (bind _notifyname (`|PlayMontage` (`self.Mesh`) "/Game/Characters/Enemies/Animations/HeavyGoblin/HeavyGoblin_Attack_End.HeavyGoblin_Attack_End")
        (:`then`
          (set `self.ReadyToAttack` false)
          (set `self.LoopAttackAnim` false))
        (:`OnCompleted`
          (`self.FinishedAttack`))
        (:`OnNotifyBegin`
          (switch `name` _notifyname
            (:`Attack`
              (bind _outhits (`KismetSystemLibrary.SphereTraceMulti` _returnvalue_2 _returnvalue_2 75.0 "TraceTypeQuery1"))
              (for _array_element _outhits
                (if (== (`.HitActor` (`GameplayStatics.BreakHitResult` _array_element)) _returnvalue)
                  (message `/Game/Blueprints/BPI_Damage.Take Damage` _returnvalue 1 self))))))))))

(event `self.UpdateOnPlayerLost`
  (bind _mesh (`self.Mesh`))
  (set `self.LoopAttackAnim` false)
  (set `self.ReadyToAttack` false)
  (if (`self.AttackMontageStarted`)
    (`SkeletalMeshComponent.SetAnimationMode` _mesh "AnimationSingleNode")
    (`SkeletalMeshComponent.SetAnimationMode` _mesh "AnimationBlueprint")
    (set `self.AttackMontageStarted` false)
    (`AIController.K2_ClearFocus` (`AIBlueprintHelperLibrary.GetAIController` self))
    (`self.UpdateState` "NewEnumerator0")))

(fn `UserConstructionScript`
  (`parent.UserConstructionScript`))
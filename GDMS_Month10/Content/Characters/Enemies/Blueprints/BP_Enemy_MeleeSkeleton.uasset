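; Melee skeleton enemy Blueprint that supplies the attack and alert animation behavior, signaling when each montage completes.
; During the attack montage, Start and End notifies start and pause a looping timer that sphere-traces at the right hand socket.
; Each trace hit on the player sends a damage message, with no guard against repeat hits in one swing.
; The construction script makes the shoulder and hat meshes follow the main mesh's pose.
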(event `/Game/Interfaces/I_Enemy.DefaultAttack`
  (bind _notifyname (`|PlayMontage` (`self.Mesh`) "/Game/Characters/Enemies/Animations/MeleeSkeleton/MeleeSkeleton_Attack_Montage.MeleeSkeleton_Attack_Montage")
    (:`OnCompleted`
      (`self.FinishedAttack`))
    (:`OnNotifyBegin`
      (switch `name` _notifyname
        (:`Start`
          (bind _returnvalue (`KismetSystemLibrary.K2_SetTimerDelegate` (delegate `StartAttack`) 0.075 true)))
        (:`End`
          (`KismetSystemLibrary.K2_PauseTimerHandle` _returnvalue))))))

(event `StartAttack`
  (bind _returnvalue (`GameplayStatics.GetPlayerCharacter` 0))
  (bind _returnvalue_2 (`SceneComponent.GetSocketLocation` (`self.Mesh`) "hand_r"))
  (bind _outhits (`KismetSystemLibrary.SphereTraceMulti` _returnvalue_2 _returnvalue_2 75.0 "TraceTypeQuery1"))
  (for _array_element _outhits
    (if (== (`.HitActor` (`GameplayStatics.BreakHitResult` _array_element)) _returnvalue)
      (message `/Game/Blueprints/BPI_Damage.Take Damage` _returnvalue 1 self))))

(event `/Game/Interfaces/I_Enemy.AlertAnimation`
  (`|PlayMontage` (`self.Mesh`) (`self.AlertAnim`)
    (:`OnCompleted`
      (`self.AlertAnimFinished`))))

(fn `UserConstructionScript`
  (`parent.UserConstructionScript`)
  (`SkinnedMeshComponent.SetLeaderPoseComponent` (`self.Shoulder`) (`self.Mesh`) false false)
  (`SkinnedMeshComponent.SetLeaderPoseComponent` (`self.Hat`) (`self.Mesh`) false false))
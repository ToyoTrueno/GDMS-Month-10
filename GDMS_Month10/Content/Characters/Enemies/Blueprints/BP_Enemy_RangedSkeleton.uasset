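; Ranged skeleton enemy that shoots arrows at the player, overriding attack and hit behavior from its parent.
; DefaultAttack plays a draw montage, then a timer triggers ShootArrow, which plays the release montage, spawns an arrow from the left hand aimed at the player and signals completion afterward.
; Hit reactions set a flag that makes the next ShootArrow skip both shot and finish call.
; Construction makes quiver and hats follow the body's pose.
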(event `/Game/Interfaces/I_Enemy.DefaultAttack`
  (`|ExecutionSequence`
    (:`then_0`
      (`|PlayMontage` (`self.Mesh`) "/Game/Characters/Enemies/Animations/RangedSkeleton/RangedSkeleton_AttackStart_Montage.RangedSkeleton_AttackStart_Montage"))
    (:`then_1`
      (`KismetSystemLibrary.K2_SetTimerDelegate` (delegate `ShootArrow`) 1.0))))

(event `ShootArrow`
  (bind _returnvalue (`SceneComponent.GetSocketLocation` (`self.Mesh`) "hand_l"))
  (if (`self.HitInteruption`)
    (set `self.HitInteruption` false)
    (else
      (`|PlayMontage` (`self.Mesh`) "/Game/Characters/Enemies/Animations/RangedSkeleton/RangedSkeleton_AttackEnd_Montage.RangedSkeleton_AttackEnd_Montage"
        (:`then`
          (`|SpawnActorFromClass` "/Game/Characters/Enemies/Blueprints/BP_Enemy_Arrow.BP_Enemy_Arrow_C" (`KismetMathLibrary.MakeTransform` _returnvalue (`KismetMathLibrary.Conv_VectorToRotator` (`KismetMathLibrary.GetDirectionUnitVector` _returnvalue (`self.K2_GetActorLocation` (`GameplayStatics.GetPlayerCharacter` 0))))) "Undefined" "MultiplyWithRoot" null null))
        (:`OnCompleted`
          (`self.FinishedAttack`))))))

(event `self.HitAnimation`
  (`parent.HitAnimation`)
  (set `self.HitInteruption` true))

(fn `UserConstructionScript`
  (`parent.UserConstructionScript`)
  (`SkinnedMeshComponent.SetLeaderPoseComponent` (`self.Quiver`) (`self.Mesh`) false false)
  (`SkinnedMeshComponent.SetLeaderPoseComponent` (`self.Hat`) (`self.Mesh`) false false)
  (`SkinnedMeshComponent.SetLeaderPoseComponent` (`self.Hat2`) (`self.Mesh`) false false))
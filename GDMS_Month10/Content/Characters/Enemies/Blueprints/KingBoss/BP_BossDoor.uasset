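; BP_BossDoor is a door actor for the King boss that can be switched between a visible, blocking state and a hidden, passable one.
; ActivateDoor enables actor collision and shows the static mesh, while DeactivateDoor disables collision and hides it.
; The construction script and BeginPlay both deactivate the door, so it starts open.
; Nothing inside the Blueprint calls ActivateDoor, leaving the trigger to outside logic.
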(event `self.ReceiveBeginPlay`
  (`self.DeactivateDoor`))

(fn `ActivateDoor`
  (`self.SetActorEnableCollision` true)
  (`SceneComponent.SetVisibility` (`self.StaticMesh`) true false))

(fn `DeactivateDoor`
  (`self.SetActorEnableCollision` false)
  (`SceneComponent.SetVisibility` (`self.StaticMesh`) false false))

(fn `UserConstructionScript`
  (`self.DeactivateDoor`))
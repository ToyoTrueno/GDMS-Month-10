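; King boss enemy that starts its behavior tree when the player enters its activation box and is destroyed when its health component reports death.
; Montage notifies drive its attacks: a ground-traced AOE spawn, a projectile fired at the player, and melee using timer-looped hand sphere traces, limited to one hit per swing.
; A dodge launches it backward; attacks and dodge call AnimFinished on blend out.
; Initialize deactivates it and restores its original location.
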(event `self.ReceiveBeginPlay`
  (add `/Game/BlueprintComponents/BPC_Health.Death` (`self.BPC_Health`) (delegate `Death`)))

(event `Death`
  (`self.K2_DestroyActor`))

(event `Initialize`
  (set `self.bActivated` false)
  (`self.K2_SetActorLocation` (`self.OriginalLocation`)))

(event `/Game/Blueprints/BPI_Damage.Take Damage`
  (params (IncomingDamage :type Byte) (Source :type "Actor Object Reference"))
  (`/Game/BlueprintComponents/BPC_Health.DecreaseHealth` (`self.BPC_Health`) Source 0))

(event `self.ActivationBox.OnComponentBeginOverlap`
  (params (OverlappedComponent :type "PrimitiveComponent Object Reference") (OtherActor :type "Actor Object Reference") (OtherComp :type "PrimitiveComponent Object Reference") (OtherBodyIndex :type Integer) (bFromSweep :type Boolean) (SweepResult :type "HitResult Structure (by ref)"))
  (if (and (== OtherActor (`GameplayStatics.GetPlayerCharacter` 0)) (not (`self.bActivated`)))
    (set `self.bActivated` true)
    (message `/Game/Interfaces/BPI_BossController.RunBT` (`AIBlueprintHelperLibrary.GetAIController` self) (`self.BehaviorTree`))))

(event `/Game/Interfaces/BPI_Boss.AOEAttack`
  (bind _returnvalue (+ (`self.K2_GetActorLocation`) (* (`self.GetActorForwardVector`) 200.0)))
  (bind _notifyname (`|PlayMontage` (`self.Mesh`) "/Game/Characters/Enemies/Animations/KingBoss/KingBoss_JumpingAttack_Montage.KingBoss_JumpingAttack_Montage")
    (:`OnBlendOut`
      (`self.AnimFinished`))
    (:`OnNotifyBegin`
      (switch `name` _notifyname
        (:`Attack`
          (bind _outhit (`KismetSystemLibrary.LineTraceSingle` _returnvalue (- _returnvalue (0.0 0.0 1000.0)) "TraceTypeQuery1"))
          (`|SpawnActorFromClass` "/Game/Characters/Enemies/Blueprints/KingBoss/BP_KingBoss_AOEAttack.BP_KingBoss_AOEAttack_C" (`KismetMathLibrary.MakeTransform` (`.ImpactPoint` (`GameplayStatics.BreakHitResult` _outhit))) "Undefined" "MultiplyWithRoot" null null))))))

(event `/Game/Interfaces/BPI_Boss.SpinAttack`
  (bind _notifyname (`|PlayMontage` (`self.Mesh`) "/Game/Characters/Enemies/Animations/KingBoss/KingBoss_ProjectileAttack.KingBoss_ProjectileAttack")
    (:`OnBlendOut`
      (`self.AnimFinished`))
    (:`OnNotifyBegin`
      (switch `name` _notifyname
        (:`Spawn`
          (`/Game/Interfaces/BPI_Boss.Projectile`))))))

(event `/Game/Interfaces/BPI_Boss.Projectile`
  (bind _returnvalue (`self.K2_GetActorLocation`))
  (`|SpawnActorFromClass` "/Game/Characters/Enemies/Blueprints/KingBoss/BP_KingBoss_Projectile.BP_KingBoss_Projectile_C" (`KismetMathLibrary.MakeTransform` _returnvalue (`KismetMathLibrary.Conv_VectorToRotator` (`KismetMathLibrary.Normal` (- (`self.K2_GetActorLocation` (`GameplayStatics.GetPlayerCharacter` 0)) _returnvalue)))) "Undefined" "MultiplyWithRoot" null null))

(event `/Game/Interfaces/BPI_Boss.MeleeAttack`
  (bind _notifyname (`|PlayMontage` (`self.Mesh`) "/Game/Characters/Enemies/Animations/KingBoss/KingBoss_Melee_Montage.KingBoss_Melee_Montage")
    (:`OnBlendOut`
      (`self.AnimFinished`))
    (:`OnNotifyBegin`
      (switch `name` _notifyname
        (:`Start`
          (`|ExecutionSequence`
            (:`then_0`
              (`self.Reset Do Once`))
            (:`then_1`
              (`self.Trace`))
            (:`then_2`
              (bind _returnvalue (`KismetSystemLibrary.K2_SetTimerDelegate` (delegate `Trace`) 0.05 true)))))
        (:`End`
          (`KismetSystemLibrary.K2_PauseTimerHandle` _returnvalue))))))

(event `Trace`
  (bind _returnvalue (`GameplayStatics.GetPlayerCharacter` 0))
  (bind _outhits (`KismetSystemLibrary.SphereTraceMulti` (`SceneComponent.GetSocketLocation` (`self.Mesh`) "hand_r") (`SceneComponent.K2_GetComponentLocation` (`self.Sphere`)) 30.0 "TraceTypeQuery1"))
  (for _array_element _outhits
    (if (== (`.HitActor` (`GameplayStatics.BreakHitResult` _array_element)) _returnvalue)
      (`/Engine/EditorBlueprintResources/StandardMacros.DoOnce` false :!label _label
        (:`Completed`
          (message `/Game/Blueprints/BPI_Damage.Take Damage` _returnvalue 1 self))))))

(event `Reset Do Once`
  (goto _label :!via `Reset`))

(event `/Game/Interfaces/BPI_Boss.Dodge`
  (`|PlayMontage` (`self.Mesh`) "/Game/Characters/Enemies/Animations/KingBoss/KingBoss_Dodge_Montage.KingBoss_Dodge_Montage"
    (:`then`
      (`self.LaunchCharacter` (+ (* (`self.GetActorForwardVector`) -500.0) (0.0 0.0 250.0)) true true))
    (:`OnBlendOut`
      (`self.AnimFinished`))))

(fn `GetEnemyStates`
  (returns (EnemyState :type "/Game/Characters/Enemies/Enums/E_EnemyStates Enum") (IdleType :type "/Game/Characters/Enemies/Enums/E_IdleTypes Enum"))
  (return "NewEnumerator0" "NewEnumerator0"))

(fn `GetPatrolPoints`
  (returns (PatrolPoints :type "Array of Vector Structure"))
  (return))

(fn `GetWanderValues`
  (returns (Center :type "Vector Structure") (Radius :type "Float (double-precision)"))
  (return (0.0 0.0 0.0) 0.0))

(fn `IsPlayerSensed?`
  (returns (Yes :type Boolean))
  (return false))

(fn `UserConstructionScript`
  (set `self.OriginalLocation` (`self.K2_GetActorLocation`)))
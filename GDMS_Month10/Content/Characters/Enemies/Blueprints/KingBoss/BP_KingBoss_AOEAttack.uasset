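; BP_KingBoss_AOEAttack is the actor for the King boss's area-of-effect attack, dealing damage to the player.
; A Box overlap sends the player character a damage message for one point of damage.
; The Box is destroyed one second after BeginPlay, limiting the damage window, while the actor destroys itself when its Niagara effect finishes.
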(event `self.ReceiveBeginPlay`
  (add `NiagaraComponent.OnSystemFinished` (`self.Niagara`) (delegate `Destroy`))
  (`KismetSystemLibrary.Delay` 1.0)
  (`ActorComponent.K2_DestroyComponent` (`self.Box`)))

(event `Destroy`
  (params (PSystem :type "NiagaraComponent Object Reference"))
  (`self.K2_DestroyActor`))

(event `self.Box.OnComponentBeginOverlap`
  (params (OverlappedComponent :type "PrimitiveComponent Object Reference") (OtherActor :type "Actor Object Reference") (OtherComp :type "PrimitiveComponent Object Reference") (OtherBodyIndex :type Integer) (bFromSweep :type Boolean) (SweepResult :type "HitResult Structure (by ref)"))
  (bind _returnvalue (`GameplayStatics.GetPlayerCharacter` 0))
  (if (== OtherActor _returnvalue)
    (message `/Game/Blueprints/BPI_Damage.Take Damage` _returnvalue 1 self)))

(fn `UserConstructionScript`)
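; King boss projectile actor that damages the player on contact.
; A Box overlap with player 0's character sends an interface TakeDamage message, then disables the box's collision so it stops registering further hits.
; The actor's lifetime follows its Niagara effect: BeginPlay binds the system-finished event to destroy the actor, so a hit does not remove it.
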(event `self.ReceiveBeginPlay`
  (add `NiagaraComponent.OnSystemFinished` (`self.Niagara`) (delegate `Destroy`)))

(event `Destroy`
  (params (PSystem :type "NiagaraComponent Object Reference"))
  (`self.K2_DestroyActor`))

(event `self.Box.OnComponentBeginOverlap`
  (params (OverlappedComponent :type "PrimitiveComponent Object Reference") (OtherActor :type "Actor Object Reference") (OtherComp :type "PrimitiveComponent Object Reference") (OtherBodyIndex :type Integer) (bFromSweep :type Boolean) (SweepResult :type "HitResult Structure (by ref)"))
  (bind _returnvalue (`GameplayStatics.GetPlayerCharacter` 0))
  (if (== OtherActor _returnvalue)
    (message `/Game/Blueprints/BPI_Damage.Take Damage` _returnvalue 1 null)
    (`PrimitiveComponent.SetCollisionEnabled` (`self.Box`) "NoCollision")))

(fn `UserConstructionScript`)
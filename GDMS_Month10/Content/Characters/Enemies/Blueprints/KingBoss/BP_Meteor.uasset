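; BP_Meteor is a meteor area attack, filed under the KingBoss enemy, that damages the player at its spawn location.
; On BeginPlay it plays a falling sound while a timeline widens the Cylinder from zero to its original footprint, then spawns a Niagara effect.
; After a short delay it plays the explosion, sphere-traces to damage the player once, and removes the Cylinder.
; The actor destroys itself when the effect finishes.
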(event `self.ReceiveBeginPlay`
  (bind _returnvalue (`self.K2_GetActorLocation`))
  (bind _returnvalue_2 (`GameplayStatics.GetPlayerCharacter` 0))
  (`|ExecutionSequence`
    (:`then_0`
      (bind _returnvalue_3 (`GameplayStatics.SpawnSoundAtLocation` "/Game/Characters/Enemies/BossSounds/MeteorFalling.MeteorFalling" (`self.K2_GetActorLocation`) (struct) 1.0 1.0 0.0 null null))
      (bind _output_get (set `self.FallingSound` _returnvalue_3))
      (`AudioComponent.Play` _output_get 0.0))
    (:`then_1`
      (bind (_direction _lerp) (`Timeline|TL_Grow` :!via `PlayFromStart`)
        (:`Update`
          (bind (_returnvalue_x _returnvalue_y) (`KismetMathLibrary.BreakVector` (`KismetMathLibrary.VLerp` (0.0 0.0 0.0) (`self.OriginalScale`) _lerp)))
          (`SceneComponent.SetWorldScale3D` (`self.Cylinder`) (`KismetMathLibrary.MakeVector` _returnvalue_x _returnvalue_y (.z (`self.OriginalScale`)))))
        (:`Finished`
          (`|ExecutionSequence`
            (:`then_0`
              (bind _returnvalue_4 (`NiagaraFunctionLibrary.SpawnSystemAtLocation` "/Game/sA_Megapack_v1/sA_StylizedAttacksPack/FX/NiagaraSystems/NS_AOE_Meteor_1.NS_AOE_Meteor_1" (`self.K2_GetActorLocation`)))
              (add `NiagaraComponent.OnSystemFinished` _returnvalue_4 (delegate `Finished`)))
            (:`then_1`
              (`KismetSystemLibrary.Delay` 1.0)
              (`|ExecutionSequence`
                (:`then_0`
                  (`AudioComponent.Stop` (`self.FallingSound`))
                  (`GameplayStatics.PlaySoundAtLocation` "/Game/Characters/Enemies/BossSounds/meteorexplode.meteorexplode" (`self.K2_GetActorLocation`) (struct) 1.0 1.0 0.0 null null null null)
                  (bind _outhits (`KismetSystemLibrary.SphereTraceMulti` _returnvalue _returnvalue 100.0 "TraceTypeQuery1"))
                  (for _array_element _outhits
                    (if (== (`.HitActor` (`GameplayStatics.BreakHitResult` _array_element)) _returnvalue_2)
                      (`/Engine/EditorBlueprintResources/StandardMacros.DoOnce` false
                        (:`Completed`
                          (message `/Game/Blueprints/BPI_Damage.Take Damage` _returnvalue_2 1 null))))))
                (:`then_1`
                  (`ActorComponent.K2_DestroyComponent` (`self.Cylinder`)))))))))))

(event `Finished`
  (params (PSystem :type "NiagaraComponent Object Reference"))
  (`self.K2_DestroyActor`))

(fn `UserConstructionScript`
  (set `self.OriginalScale` (`SceneComponent.K2_GetComponentScale` (`self.Cylinder`))))
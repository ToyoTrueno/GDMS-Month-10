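; Friendly goblin NPC character that comes in Warrior, Wizard and Ice variants.
; The construction script uses the Type variable to pick the body material and the skeletal meshes for hat, torso, waist, arms and legs.
; On BeginPlay it runs the parent logic, then flags its health component as invincible.
; The Tick, overlap and SetMaxWalkSpeed events are empty.
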(event `self.ReceiveBeginPlay`
  (`parent.ReceiveBeginPlay`)
  (set `/Game/BlueprintComponents/BPC_Health.Invincible` true (`self.BPC_Health`)))

(event `self.ReceiveTick`
  (params (DeltaSeconds :type "Float (single-precision)")))

(event `/Game/Interfaces/I_Enemy.SetMaxWalkSpeed`)

(fn `UserConstructionScript`
  (`parent.UserConstructionScript`)
  (`PrimitiveComponent.SetMaterial` (`self.Mesh`) 0 (select `/Game/Characters/FriendlyNPC/Goblin/E_GoblinType` (`self.Type`) :`NewEnumerator0` "/Game/Characters/Goblin/Material/Goblin_Base/Mat_Goblin_green.Mat_Goblin_green" :`NewEnumerator1` "/Game/Characters/Goblin/Material/Goblin_Base/Mat_Goblin_red.Mat_Goblin_red" :`NewEnumerator2` "/Game/Characters/Goblin/Material/Goblin_Base/Mat_Goblin_ice.Mat_Goblin_ice" :!type "MaterialInterface Object Reference"))
  (`SkeletalMeshComponent.SetSkeletalMeshAsset` (`self.Hat`) (select `/Game/Characters/FriendlyNPC/Goblin/E_GoblinType` (`self.Type`) :`NewEnumerator0` "/Game/Characters/Goblin/Mesh/Goblin_armor/SK_Head_Helmet.SK_Head_Helmet" :`NewEnumerator1` "/Game/Characters/Goblin/Mesh/Goblin_Wizard/SK_Wizard_Hat.SK_Wizard_Hat" :`NewEnumerator2` "/Game/Characters/Goblin/Mesh/Goblin_ice/SK_Head_ice.SK_Head_ice" :!type "SkeletalMesh Object Reference"))
  (`SkeletalMeshComponent.SetSkeletalMeshAsset` (`self.Torso`) (select `/Game/Characters/FriendlyNPC/Goblin/E_GoblinType` (`self.Type`) :`NewEnumerator0` "/Game/Characters/Goblin/Mesh/Goblin_armor/SK_Goblin_Body_Armor.SK_Goblin_Body_Armor" :`NewEnumerator1` "/Game/Characters/Goblin/Mesh/Goblin_Wizard/SK_Wizard_Cloak.SK_Wizard_Cloak" :`NewEnumerator2` "/Game/Characters/Goblin/Mesh/Goblin_armor_ice/SK_Goblin_Body_Armor_ice.SK_Goblin_Body_Armor_ice" :!type "SkeletalMesh Object Reference"))
  (`SkeletalMeshComponent.SetSkeletalMeshAsset` (`self.Waist`) (select `/Game/Characters/FriendlyNPC/Goblin/E_GoblinType` (`self.Type`) :`NewEnumerator0` "/Game/Characters/Goblin/Mesh/Goblin_armor/SK_Goblin_skirt.SK_Goblin_skirt" :`NewEnumerator1` "/Game/Characters/Goblin/Mesh/Goblin_Wizard/SK_Wizard_Pants.SK_Wizard_Pants" :`NewEnumerator2` "/Game/Characters/Goblin/Mesh/Goblin_armor_ice/SK_Goblin_skirt_ice.SK_Goblin_skirt_ice" :!type "SkeletalMesh Object Reference"))
  (`SkeletalMeshComponent.SetSkeletalMeshAsset` (`self.Arms`) (select `/Game/Characters/FriendlyNPC/Goblin/E_GoblinType` (`self.Type`) :`NewEnumerator0` "/Game/Characters/Goblin/Mesh/Goblin_armor/SK_Goblin_Bracers.SK_Goblin_Bracers" :`NewEnumerator1` "/Game/Characters/Goblin/Mesh/Goblin_Wizard/SK_Wizard_Bracers.SK_Wizard_Bracers" :`NewEnumerator2` "/Game/Characters/Goblin/Mesh/Goblin_ice/SK_Shoulder_ice.SK_Shoulder_ice" :!type "SkeletalMesh Object Reference"))
  (`SkeletalMeshComponent.SetSkeletalMeshAsset` (`self.Legs`) (select `/Game/Characters/FriendlyNPC/Goblin/E_GoblinType` (`self.Type`) :`NewEnumerator0` "/Game/Characters/Goblin/Mesh/Goblin_armor/SK_Goblin_Leg_Armor.SK_Goblin_Leg_Armor" :`NewEnumerator1` "/Game/Characters/Goblin/Mesh/Goblin_Wizard/SK_Wizard_Scroll.SK_Wizard_Scroll" :`NewEnumerator2` "/Game/Characters/Goblin/Mesh/Goblin_ice/SK_Top_Leg_ice.SK_Top_Leg_ice" :!type "SkeletalMesh Object Reference")))